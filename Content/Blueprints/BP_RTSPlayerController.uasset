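; RTS player controller that handles camera movement and unit selection input through Enhanced Input.
; It moves the RTS pawn by control rotation and feeds mouse positions to the HUD, which draws the selection box and is told to select on release.
; Click selection clears the unit manager unless shift is held, then sphere-traces from the cursor hit toward the camera.
; The final BPI_Selectable check on the traced unit currently triggers nothing.
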(event Custom|Do%20Selection%20Command
  (bind (_hit _location) (CallFunction|GetPawnUnderCursor))
  ;[0.15 0.15 0.15 0.5] Trigger Selection Command / Sphere Trace from camera -> floor to select stuff
  (if (Variables|Default|GetShiftMod)
    _
    (else
      (Default|DeselectAll (Variables|Default|GetUnitManager))))
  (if _hit
    (Variables|Default|SetCachedSelection _location)
    (bind _outhit (Collision|SphereTraceForObjects (Variables|Default|GetCachedSelection) (Transformation|GetWorldLocation (Variables|/Game/Blueprints/BP_RTSPawn.BP_RTSPawn_C|GetCamera (Variables|Default|GetControlledPawn))) (Variables|Default|GetInteractionRadius) (Utilities|Array|MakeArray "ObjectTypeQuery3") false 0 "ForDuration"))
    (if (.bBlockingHit (Collision|BreakHitResult _outhit))
      (bind _output_get (Variables|ObjectTracking|SetTarget%20Unit (.HitActor (Collision|BreakHitResult _outhit))))
      (if (Utilities|DoesObjectImplementInterface (Actor|GetComponentbyClass _output_get "/Game/Blueprints/Components/SelectionComponent.SelectionComponent_C") "/Game/Blueprints/Interfaces/BPI_Selectable.BPI_Selectable_C")
        _))))

(event Input|EnhancedActionEvents|EnhancedInputActionIA_Select
  (params (ActionValue :type Boolean) (ElapsedSeconds :type Float%20%28double-precision%29) (TriggeredSeconds :type Float%20%28double-precision%29) (InputAction :type Input%20Action%20Object%20Reference :default "/Game/Inputs/Actions/IA_Select.IA_Select"))
  ;[0.15 0.15 0.15 0.5] Trigger Selection Command / Sphere Trace from camera -> floor to select stuff
  (CallFunction|DoSelectionCommand))

(event Input|EnhancedActionEvents|EnhancedInputActionIA_SelectionBox
  (params (ActionValue :type Boolean) (ElapsedSeconds :type Float%20%28double-precision%29) (TriggeredSeconds :type Float%20%28double-precision%29) (InputAction :type Input%20Action%20Object%20Reference :default "/Game/Inputs/Actions/IA_SelectionBox.IA_SelectionBox"))
  ;[0.15 0.15 0.15 0.5] Selection Box Logic - Select / Drag Select
  (:Started
    (bind _mouse_pos (CallFunction|GetMouseLocation))
    (bind _output_get (Variables|MousePosition|SetStartingSelectionPos _mouse_pos))
    (Class|BPIRTS|DragSelectUpdate(Message) (Variables|Default|GetHUD) _output_get "(X=0.000000,Y=0.000000)" "(X=0.000000,Y=0.000000)" false false) ; This is only here for now so the debug HUD can set the "Start Pos".
  )
  (:Ongoing
    (bind _mouse_pos_2 (CallFunction|GetMouseLocation))
    (bind _output_get_2 (Variables|MousePosition|SetCurrentSelectionPos (Math|Vector2D|MakeVector2D (.x _mouse_pos_2) (.y _mouse_pos_2))))
    (Class|BPIRTS|DragSelectUpdate(Message) (Variables|Default|GetHUD) (Variables|MousePosition|GetStartingSelectionPos) (Math|Vector2D|MakeVector2D (.x _output_get_2) (.y _output_get_2)) (Math|Vector2D|MakeVector2D (- (.x _output_get_2) (.x (Variables|MousePosition|GetStartingSelectionPos))) (- (.y _output_get_2) (.y (Variables|MousePosition|GetStartingSelectionPos)))) true false))
  (:Canceled
    (Class|BPIRTS|DragSelectUpdate(Message) :self (Variables|Default|GetHUD) :SelectUnits true :!label _label))
  (:Completed
    (goto _label)))

(event Input|EnhancedActionEvents|EnhancedInputActionIA_MoveCamera
  (params (ActionValue :type Vector%202D%20Structure) (ElapsedSeconds :type Float%20%28double-precision%29) (TriggeredSeconds :type Float%20%28double-precision%29) (InputAction :type Input%20Action%20Object%20Reference :default "/Game/Inputs/Actions/IA_MoveCamera.IA_MoveCamera"))
  (bind _returnvalue (Pawn|GetControlRotation :!class /Script/Engine.Controller))
  (bind _controlledpawn (Variables|Default|GetControlledPawn))
  ;[0.15 0.15 0.15 0.5] Logic for moving around the camera
  (Pawn|Input|AddMovementInput _controlledpawn (Math|Vector|GetForwardVector (Math|Rotator|MakeRotator (.roll _returnvalue) 0.0 (.yaw _returnvalue))) (+ (.x ActionValue) (.y ActionValue)) false)
  (Pawn|Input|AddMovementInput _controlledpawn (Math|Vector|GetRightVector (Math|Rotator|MakeRotator 0.0 0.0 (.yaw (Pawn|GetControlRotation :!class /Script/Engine.Controller)))) (- (.x ActionValue) (.y ActionValue)) false))

(event Input|EnhancedActionEvents|EnhancedInputActionIA_ShiftMod
  (params (ActionValue :type Boolean) (ElapsedSeconds :type Float%20%28double-precision%29) (TriggeredSeconds :type Float%20%28double-precision%29) (InputAction :type Input%20Action%20Object%20Reference :default "/Game/Inputs/Actions/Modifiers/IA_ShiftMod.IA_ShiftMod"))
  (:Started
    (Variables|Default|SetShiftMod true))
  (:Completed
    (Variables|Default|SetShiftMod false)))

(event EventBeginPlay
  (bind _returnvalue (PlayerController|LocalPlayerSubsystems|GetEnhancedInputLocalPlayerSubsystem))
  (Utilities|FlowControl|Sequence
    (:then_0
      (bind _asbp_rtspawn (Utilities|Casting|CastToBP_RTSPawn (Pawn|GetControlledPawn)))
      (Variables|Default|SetControlledPawn _asbp_rtspawn)
      (Variables|Default|SetHUD (HUD|GetHUD)))
    (:then_1
      (Utilities|IsValid _returnvalue
        (:Is%20Valid
          (Input|AddMappingContext _returnvalue "/Game/Inputs/IMC_RTS.IMC_RTS" 0 "(bIgnoreAllPressedKeysUntilRelease=True,bForceImmediately=False,bNotifyUserSettings=False)"))))
    (:then_2
      (bind (_unitmanager _is_valid) (CallFunction|GetUnitManager))
      (if _is_valid
        (Variables|Default|SetUnitManager _unitmanager)))))

(fn ConstructionScript)

(fn GetMouseLocation
  (bind _returnvalue (Game|GetPlayerController 0))
  (bind (_locationx _locationy) (Game|Player|GetMousePosition _returnvalue))
  (return (Math|Vector2D|MakeVector2D _locationx _locationy)))

(fn GetPawnUnderCursor
  (bind _array (Utilities|Array|MakeArray "ObjectTypeQuery3"))
  (bind _hitresult (Class|PlayerController|GetHitResultUnderCursorforObjects _array false))
  (bind (_bblockinghit _binitialoverlap _time _distance _location) (Collision|BreakHitResult _hitresult))
  (return _bblockinghit _location))