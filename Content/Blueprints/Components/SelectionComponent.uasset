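; Selection component that makes its owning unit selectable and highlightable, registering it with the Unit Manager on BeginPlay.
; The owner's cursor-over events send highlight messages, while select, deselect and highlight events guard state flags and broadcast changes through dispatchers.
; Tick broadcasts the owner's position and whether it is moving.
; Separate functions toggle selection and highlight decal visibility.
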(event Custom|OnBeginCursorOver
  (params (TouchedActor :type Actor%20Object%20Reference))
  ;[0.15 0.15 0.15 0.5] Highlight On Hover Logic
  (Class|BPISelectable|HighlightUnit(Message) self))

(event Custom|OnEndCursorOver
  (params (TouchedActor :type Actor%20Object%20Reference))
  ;[0.15 0.15 0.15 0.5] Highlight On Hover Logic
  (Class|BPISelectable|UnhighlightUnit(Message) self))

(event EventBeginPlay
  (Utilities|FlowControl|Sequence
    (:then_0
      ;[0.15 0.15 0.15 0.5] Register Unit w/ Unit Manager
      (bind (_unitmanager _is_valid) (CallFunction|GetUnitManager))
      (if _is_valid
        (bind _output_get (Variables|Default|SetUnitManager _unitmanager))
        (Default|RegisterUnit _output_get self)))
    (:then_1
      ;[0.15 0.15 0.15 0.5] Setup Select/Highlight Decals
      (Variables|Default|SetOwner (Components|GetOwner)))
    (:then_2
      ;[0.15 0.15 0.15 0.5] Bind to Unit's On Begin/End Cursor Events
      (EventDispatchers|BindEventtoOnBeginCursorOver (Variables|Default|GetOwner) (EventDispatchers|CreateEvent :!event Custom|OnBeginCursorOver))
      (EventDispatchers|BindEventtoOnEndCursorOver (Variables|Default|GetOwner) (EventDispatchers|CreateEvent :!event Custom|OnEndCursorOver)))))

(event EventTick
  (params (DeltaSeconds :type Float%20%28single-precision%29))
  (bind _self self)
  (bind _owner (Variables|Default|GetOwner))
  (bind _output_get (Variables|Default|SetIsMoving (> (Math|Vector|VectorLength (Transformation|GetVelocity _owner)) 0.0)))
  (Default|CallUnitMoving _self _output_get _self (Transformation|GetActorLocation _owner)))

(event EventSelectUnit
  ;[0.15 0.15 0.15 0.5] Select Unit Logic - also handles unhighlighting
  (Utilities|FlowControl|Sequence
    (:then_0
      (if (Variables|Default|GetIsHighlighted)
        (Default|UnhighlightUnit self)))
    (:then_1
      (if (not (Variables|Default|GetIsSelected))
        (Variables|Default|SetIsSelected true)
        (Default|CallUnitSelected self)))))

(event EventDeselectUnit
  ;[0.15 0.15 0.15 0.5] Deselect Unit Logic - also handles unhighlighting
  (Utilities|FlowControl|Sequence
    (:then_0
      (if (Variables|Default|GetIsHighlighted)
        (Default|UnhighlightUnit self)))
    (:then_1
      (if (Variables|Default|GetIsSelected)
        (Variables|Default|SetIsSelected false)
        (Default|CallUnitDeselected self)))))

(event EventHighlightUnit
  ;[0.15 0.15 0.15 0.5] Highlight Unit Logic
  (if (and (not (Variables|Default|GetIsHighlighted)) (not (Variables|Default|GetIsSelected)))
    (Variables|Default|SetIsHighlighted true)
    (Default|CallUnitHighlighted self)))

(event EventUnhighlightUnit
  ;[0.15 0.15 0.15 0.5] Unhighlight Unit Logic
  (if (and (Variables|Default|GetIsHighlighted) (not (Variables|Default|GetIsSelected)))
    (Variables|Default|SetIsHighlighted false)
    (Default|CallUnitUnhighlighted self)))

(fn SetSelectionDecal
  (params (ShowDecal :type Boolean))
  (Rendering|SetVisibility (Variables|Default|GetSelectionDecal) ShowDecal false))

(fn SetHighlightDecal
  (params (ShowDecal :type Boolean))
  (Rendering|SetVisibility (Variables|Default|GetHighlightDecal) ShowDecal false))