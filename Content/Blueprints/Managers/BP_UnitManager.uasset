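; Unit manager that registers units, tracks which are highlighted and selected, and draws selection circles under selected units.
; It registers itself on the game mode, binds to each registered unit's highlight and selection events, and rebroadcasts changes to its lists.
; Each tick it feeds selected units' owner locations into one Niagara system's position array, so a single effect renders every circle.
; Batch functions deselect all or select all highlighted units.
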(event Custom|UnitHighlighted
  (params (TargetUnit :type Selection%20Component%20Object%20Reference))
  (bind _returnvalue (Utilities|Array|AddUnique (Variables|UnitArrays|GetHighlightedUnits) TargetUnit))
  (if (>= _returnvalue 0)
    (Default|CallOnUnitHighlighted)))

(event Custom|UnitUnhighlighted
  (params (TargetUnit :type Selection%20Component%20Object%20Reference))
  (bind _returnvalue (Utilities|Array|RemoveItem (Variables|UnitArrays|GetHighlightedUnits) TargetUnit))
  (if _returnvalue
    (Default|CallOnUnitUnhighlighted)))

(event Custom|UnitSelected
  (params (TargetUnit :type Selection%20Component%20Object%20Reference))
  (bind _returnvalue (Utilities|Array|AddUnique (Variables|UnitArrays|GetSelectedUnits) TargetUnit))
  (if (>= _returnvalue 0)
    (Utilities|FlowControl|Sequence
      (:then_0
        (Default|CallOnUnitSelected)))))

(event Custom|UnitDeselected
  (params (TargetUnit :type Selection%20Component%20Object%20Reference))
  (bind _returnvalue (Utilities|Array|RemoveItem (Variables|UnitArrays|GetSelectedUnits) TargetUnit))
  (if _returnvalue
    (Utilities|FlowControl|Sequence
      (:then_0
        (Default|CallOnUnitDeselected)))))

(event EventBeginPlay
  (bind _bprtsgame_mode (CallFunction|GetGameMode))
  (Variables|/Game/Blueprints/BP_RTSGameMode.BP_RTSGameMode_C|SetUnitManager _bprtsgame_mode self)
  (bind _returnvalue (Niagara|SpawnSystematLocation "/Game/Blueprints/NS_UnitCircles.NS_UnitCircles" "0, 0, 0" "0, 0, 0" "1.000000,1.000000,1.000000" false true "AutoRelease"))
  (Variables|Default|SetUnitCircleSystem _returnvalue))

(event EventTick
  (params (DeltaSeconds :type Float%20%28single-precision%29))
  (bind _unitpositions (Variables|UnitArrays|GetUnitPositions))
  (if (> (Utilities|Array|Length (Variables|UnitArrays|GetSelectedUnits)) 0)
    (for _array_element (Variables|UnitArrays|GetSelectedUnits)
      (Utilities|Array|Add (Variables|UnitArrays|GetUnitPositions) (Transformation|GetActorLocation (Components|GetOwner _array_element)))))
  (Class|NiagaraDataInterfaceArrayFunctionLibrary|SetNiagaraArrayPosition (Variables|Default|GetUnitCircleSystem) "PositionArray" _unitpositions)
  (Utilities|Array|Clear _unitpositions))

(fn ConstructionScript)

(fn RegisterUnit
  (params (UnitToRegister :type Selection%20Component%20Object%20Reference))
  (EventDispatchers|BindEventtoUnitHighlighted UnitToRegister (EventDispatchers|CreateEvent :!event Custom|UnitHighlighted))
  (EventDispatchers|BindEventtoUnitUnhighlighted UnitToRegister (EventDispatchers|CreateEvent :!event Custom|UnitUnhighlighted))
  (EventDispatchers|BindEventtoUnitSelected UnitToRegister (EventDispatchers|CreateEvent :!event Custom|UnitSelected))
  (EventDispatchers|BindEventtoUnitDeselected UnitToRegister (EventDispatchers|CreateEvent :!event Custom|UnitDeselected))
  (Utilities|Array|AddUnique (Variables|UnitArrays|GetRegisteredUnits) UnitToRegister)
  (return))

(fn DeselectAll
  (bind _output_get (LocalVariables|SetLocalSelectedUnits (Variables|UnitArrays|GetSelectedUnits)))
  (for _array_element _output_get
    (Utilities|IsValid _array_element
      (:Is%20Valid
        (Class|BPISelectable|DeselectUnit(Message) _array_element)))))

(fn SelectAllHighlighted
  (bind _output_get (LocalVariables|SetLocalHighlightedUnits (Variables|UnitArrays|GetHighlightedUnits)))
  (for _array_element _output_get
    (Utilities|IsValid _array_element
      (:Is%20Valid
        (Class|BPISelectable|SelectUnit(Message) _array_element)))))