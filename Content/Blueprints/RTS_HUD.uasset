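; RTS HUD Blueprint that creates the UI_RTS widget and handles drag-box unit selection.
; DragSelectUpdate stores the rectangle and draw/select flags and shows the start position in the widget.
; While drawing, DrawHUD renders the box, highlights Pawns' SelectionComponents inside it and unhighlights UnitManager's highlighted units that fall outside.
; When drawing stops with selection requested, UnitManager selects all highlighted units.
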(event EventDragSelectUpdate
  (params (StartPos :type Vector%202D%20Structure) (CurrentPos :type Vector%202D%20Structure) (Width%20And%20Height :type Vector%202D%20Structure) (Draw :type Boolean) (SelectUnits :type Boolean))
  (Variables|/Game/Blueprints/UI/UI_RTS.UI_RTS_C|SetStartingPos (Variables|SelectionBoxVars|GetUI) (Utilities|Text|ToText(String) StartPos))
  (Variables|SelectionBoxVars|SetSelect%20Units SelectUnits)
  (Variables|SelectionBoxVars|SetDraw Draw)
  (Variables|SelectionBoxVars|SetStart StartPos)
  (Variables|SelectionBoxVars|SetCurrent CurrentPos)
  (Variables|SelectionBoxVars|SetWidthHeight Width%20And%20Height))

(event EventBeginPlay
  (Utilities|FlowControl|Sequence
    (:then_0
      (bind _returnvalue (UserInterface|CreateWidget "/Game/Blueprints/UI/UI_RTS.UI_RTS_C" (Game|GetPlayerController 0)))
      (bind _output_get (Variables|SelectionBoxVars|SetUI _returnvalue))
      (UserInterface|Viewport|AddtoViewport _returnvalue 0))
    (:then_1
      (bind (_unitmanager _is_valid) (CallFunction|GetUnitManager))
      (if _is_valid
        (Variables|Default|SetUnitManager _unitmanager)))))

(event EventDrawHUD
  (params (SizeX :type Integer) (SizeY :type Integer))
  (bind _selectableunits (Variables|Default|GetSelectableUnits))
  (bind _start (Variables|SelectionBoxVars|GetStart))
  (bind _widthheight (Variables|SelectionBoxVars|GetWidthHeight))
  (if (Variables|SelectionBoxVars|GetDraw)
    (HUD|DrawRect "(R=0.092132,G=0.779664,B=1.000000,A=0.500000)" (.x _start) (.y _start) (.x _widthheight) (.y _widthheight))
    (for _array_element (Class|HUD|GetActorsinSelectionRectangle "/Script/Engine.Pawn" (Variables|SelectionBoxVars|GetStart) (Variables|SelectionBoxVars|GetCurrent) true false)
      (Utilities|Array|AddUnique _selectableunits (Actor|GetComponentbyClass _array_element "/Game/Blueprints/Components/SelectionComponent.SelectionComponent_C"))
      (Class|BPISelectable|HighlightUnit(Message) (Actor|GetComponentbyClass _array_element "/Game/Blueprints/Components/SelectionComponent.SelectionComponent_C")))
    (for _array_element_2 (Variables|/Game/Blueprints/Managers/BP_UnitManager.BP_UnitManager_C|GetHighlightedUnits (Variables|Default|GetUnitManager))
      (if (not (Utilities|Array|ContainsItem _selectableunits _array_element_2))
        (Class|BPISelectable|UnhighlightUnit(Message) _array_element_2)))
    (Utilities|Array|Clear _selectableunits)
    (elif (Variables|SelectionBoxVars|GetSelect%20Units)
      (Default|SelectAllHighlighted (Variables|Default|GetUnitManager))
      (Variables|SelectionBoxVars|SetSelect%20Units false))))

(fn ConstructionScript)